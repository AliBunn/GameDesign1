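; BP_GoToNextLevel is a trigger actor that sends the player to another level.
; When a BP_ThirdPersonCharacterCustom overlaps its Box and Destination is valid, it fades the camera and audio out over FadeDuration, waits that long, then opens the Destination level by object reference.
; An invalid Destination only prints a warning, and leftover open-by-name nodes are never run.
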(event `self.Box.OnComponentBeginOverlap`
  (params (OverlappedComponent :type "PrimitiveComponent Object Reference") (OtherActor :type "Actor Object Reference") (OtherComp :type "PrimitiveComponent Object Reference") (OtherBodyIndex :type Integer) (bFromSweep :type Boolean) (SweepResult :type "HitResult Structure (by ref)"))
  (cast `/Game/Blueprints/BP_ThirdPersonCharacterCustom` OtherActor)
  (bind _destination (`self.Destination`)
    (:`then`
      (`PlayerCameraManager.StartCameraFade` :`self` (`GameplayStatics.GetPlayerCameraManager` 0) :`ToAlpha` 1.0 :`Duration` (`self.Fade Duration`) :`bShouldFadeAudio` true :`bHoldWhenFinished` true) ; Need to add a delay of one sec
      (`KismetSystemLibrary.Delay` (`self.Fade Duration`))
      (`GameplayStatics.OpenLevelBySoftObjectPtr` _destination))
    (:`else`
      (`KismetSystemLibrary.PrintString` "No valid destination"))))

(fn `UserConstructionScript`)