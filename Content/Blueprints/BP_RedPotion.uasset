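; BP_RedPotion is a holdable potion item that the custom third-person character can pick up, drop or throw.
; Overlapping its sphere calls the character's TryToPickUp, and Pickup attaches the cone mesh to the hand_r socket with collision off.
; Drop detaches the cone in place with physics and collision on, while PrimaryAction also launches it forward with a mass-independent impulse and clears HeldItem.
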(event `self.Sphere.OnComponentBeginOverlap`
  (params (OverlappedComponent :type "PrimitiveComponent Object Reference") (OtherActor :type "Actor Object Reference") (OtherComp :type "PrimitiveComponent Object Reference") (OtherBodyIndex :type Integer) (bFromSweep :type Boolean) (SweepResult :type "HitResult Structure (by ref)"))
  (bind _asbp_third_person_character_custom (cast `/Game/Blueprints/BP_ThirdPersonCharacterCustom` OtherActor))
  (`/Game/Blueprints/BP_ThirdPersonCharacterCustom.TryToPickUp` _asbp_third_person_character_custom self))

(event `/Game/Blueprints/BPI_Item.Pickup`
  (params (ParentMesh :type "SkeletalMeshComponent Object Reference"))
  (`SceneComponent.K2_AttachToComponent` (`self.Cone`) ParentMesh "hand_r" "SnapToTarget" "KeepRelative" "KeepRelative" true)
  (`PrimitiveComponent.SetCollisionEnabled` (`self.Cone`) "NoCollision") ; Collide with the ground please
)

(event `/Game/Blueprints/BPI_Item.Drop`
  (bind _cone (`self.Cone`))
  (set `self.Drop Location` (`SceneComponent.K2_GetComponentLocation` _cone))
  (`SceneComponent.K2_DetachFromComponent` _cone "KeepRelative" "KeepRelative" "KeepRelative" true) ; Don't follow the hand anymore
  (`PrimitiveComponent.SetSimulatePhysics` (`self.Cone`) true) ; use gravity to fall
  (`PrimitiveComponent.SetCollisionEnabled` (`self.Cone`) "QueryAndPhysics") ; Collide with the ground please
  (`SceneComponent.K2_SetWorldLocation` (`self.Cone`) (`self.Drop Location`) false false) ; To prevent the can from going to world origin
)

(event `/Game/Blueprints/BPI_Item.PrimaryAction`
  (params (ref_thirdPersonCharCustom :type "/Game/Blueprints/BP_ThirdPersonCharacterCustom Object Reference"))
  (set `self.Drop Location` (+ (`SceneComponent.K2_GetComponentLocation` (`self.Cone`)) (* (`SceneComponent.GetForwardVector` (`Character.CapsuleComponent` (`GameplayStatics.GetPlayerCharacter` 0))) 50.0)))
  (`SceneComponent.K2_DetachFromComponent` (`self.Cone`) "KeepRelative" "KeepRelative" "KeepRelative" true) ; Don't follow the hand anymore
  (`PrimitiveComponent.SetSimulatePhysics` (`self.Cone`) true) ; use gravity to fall
  (`PrimitiveComponent.SetCollisionEnabled` (`self.Cone`) "QueryAndPhysics") ; Collide with the ground please
  (`SceneComponent.K2_SetWorldLocation` (`self.Cone`) (`self.Drop Location`) false false) ; To prevent the can from going to world origin
  (`PrimitiveComponent.AddImpulse` (`self.Cone`) (* (`self.GetActorForwardVector` (`GameplayStatics.GetPlayerCharacter` 0)) 1000.0) "None" true)
  (set `/Game/Blueprints/BP_ThirdPersonCharacterCustom.HeldItem` null ref_thirdPersonCharCustom))

(fn `UserConstructionScript`)