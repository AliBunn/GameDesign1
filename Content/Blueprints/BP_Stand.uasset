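; BP_Stand is a musical stand that plays a note and brightens its material, with unfinished interaction for a turn-based exchange.
; BeginPlay assigns the sound, and PlayNote plays it, raises DynMat's Intensity and ends on a short delay without resetting it.
; OnInteract checks the actor's interface and player turn but triggers nothing.
; The capsule's dynamic material and color setup is disconnected from the construction script, so DynMat is never created here.
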(event `self.ReceiveBeginPlay`
  (`AudioComponent.SetSound` (`self.Audio`) (`self.New Sound`)))

(event `/Game/Blueprints/BP_Interactable.OnInteract`
  (params (Actor :type "Actor Object Reference"))
  (if (`KismetSystemLibrary.DoesImplementInterface` Actor)
    ;[1 1 1] IsPlayerTurn
    (if true
      _)))

(event `PlayNote`
  (`AudioComponent.Play` (`self.Audio`) 0.0)
  (`MaterialInstanceDynamic.SetScalarParameterValue` (`self.DynMat`) "Intensity" 2.5)
  (`KismetSystemLibrary.Delay` 0.65))

(fn `UserConstructionScript`)