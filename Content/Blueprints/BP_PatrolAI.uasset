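; BP_PatrolAI is an AI pawn that continually chases the first player character, despite its patrol naming.
; BeginPlay starts MoveTo, which runs AIMoveTo on itself toward the player and re-issues it after a short delay on success or failure.
; Patrol logic is unfinished: BeginPlay fetches tagged test-map patrol points without using them and calls an empty GotoDestination event.
; Print strings serve as debug output.
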(event `self.ReceiveBeginPlay`
  (`self.Move To`)
  (`GameplayStatics.GetAllActorsOfClassWithTag` null "PatrolPoint-TestMap")
  (`KismetSystemLibrary.PrintString` "Hello")
  (`self.Go to Destination`))

(event `Go to Destination`)

(event `Move To`
  (`|AIMoveTo` self (0.0 0.0 0.0) (`GameplayStatics.GetPlayerCharacter` 0) ; Move ourselves to the players location, constantly updating, and stopping 2 meters away
    (:`OnSuccess`
      (`KismetSystemLibrary.PrintString` "Arrived at Destination"))
    (:`OnFail`
      (`KismetSystemLibrary.PrintString` "Failed to get to Destination")))
  (`KismetSystemLibrary.Delay` 0.2)
  (`self.Move To`))

(fn `UserConstructionScript`)