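; BP_Apple is an apple ingredient that bobs up and down and adds to the player's apple count on overlap.
; A timeline started on BeginPlay raises the apple half mesh, and a FlipFlop on Finished alternates Reverse and Play to loop the motion.
; Sphere overlap by BP_ThirdPersonCharacterCustom increments TotalApples and prints the count, without destroying or hiding the apple.
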(event `Play`
  (bind (_direction _newtrack_0) (`Timeline|Timeline` :!label _label)
    (:`Update`
      (`SceneComponent.K2_SetRelativeLocation` (`self.apple_apple_half_1`) (`KismetMathLibrary.MakeVector` 0.0 0.0 (`KismetMathLibrary.Lerp` 0.0 25.0 _newtrack_0)) false false))
    (:`Finished`
      (`/Engine/EditorBlueprintResources/StandardMacros.FlipFlop`
        (:`A`
          (`self.Reverse`))
        (:`B`
          (`self.Play`))))))

(event `self.ReceiveBeginPlay`
  (goto _label))

(event `Reverse`
  (goto _label :!via `Reverse`))

(event `self.Sphere1.OnComponentBeginOverlap`
  (params (OverlappedComponent :type "PrimitiveComponent Object Reference") (OtherActor :type "Actor Object Reference") (OtherComp :type "PrimitiveComponent Object Reference") (OtherBodyIndex :type Integer) (bFromSweep :type Boolean) (SweepResult :type "HitResult Structure (by ref)"))
  (bind _asbp_third_person_character_custom (cast `/Game/Blueprints/BP_ThirdPersonCharacterCustom` OtherActor))
  (bind _result (`/Engine/EditorBlueprintResources/StandardMacros.IncrementInt` (`.totalApples_6_D2EF199B4463671DE00084A70336A1A5` (break `/Game/Blueprints/BP_Ingreidents` (`/Game/Blueprints/BP_ThirdPersonCharacterCustom.Ingreidents` _asbp_third_person_character_custom)))) ; Means to add one
    (:`  `
      (`KismetSystemLibrary.PrintString` (`KismetStringLibrary.Conv_IntToString` _result) true true (struct :`G` 0.66 :`B` 1.0 :`A` 1.0) 3.0))))

(fn `UserConstructionScript`)